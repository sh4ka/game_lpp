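; Player controller for a falling-block puzzle, steering a quad of two-color blocks held by LPPGameMode_BP.
; Input shifts, drops or rotates the quad, with rotation cycling colors between blocks instead of moving actors.
; A re-armed timer drives falling; line traces against grid and blocks gate moves and let left and right halves descend independently.
; When neither half can fall, it triggers match checks and spawns the next quad.
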(event `self.ReceiveBeginPlay`
  (bind _gamemode (`self.GameMode`))
  (`/Game/LPPGameMode_BP.SpawnNewQuad` _gamemode)
  (`KismetSystemLibrary.K2_SetTimer` null "FallDownOneSpace" (`/Game/LPPGameMode_BP.TimeBetweenAutomaticFalls` _gamemode)))

(event `InputAction|MoveLeft`
  (params (Key :type "Key Structure"))
  (:`Pressed`
    (if (not (`/Game/LPPGameMode_BP.bIsQuadDroppingFaster` (`self.GameMode`)))
      (bind _bcanmove (`self.CanMoveLeft`))
      (if _bcanmove
        (`self.MoveBlocksLeft`)))))

(event `InputAction|MoveRight`
  (params (Key :type "Key Structure"))
  (:`Pressed`
    (if (not (`/Game/LPPGameMode_BP.bIsQuadDroppingFaster` (`self.GameMode`)))
      (bind _bcanmove (`self.CanMoveRight`))
      (if _bcanmove
        (`self.MoveBlocksRight`)))))

(event `InputAction|RotateClockwise`
  (params (Key :type "Key Structure"))
  (:`Pressed`
    (if (not (`/Game/LPPGameMode_BP.bIsQuadDroppingFaster` (`self.GameMode`)))
      (`self.RotateBlocksCW`))))

(event `InputAction|RotateCounterclockwise`
  (params (Key :type "Key Structure"))
  (:`Pressed`
    (if (not (`/Game/LPPGameMode_BP.bIsQuadDroppingFaster` (`self.GameMode`)))
      (`self.RotateBlocksCCW`))))

(event `InputAction|MoveDown`
  (params (Key :type "Key Structure"))
  (bind _gamemode (`self.GameMode`))
  (:`Pressed`
    (if (`/Game/LPPGameMode_BP.bIsQuadDroppingFaster` _gamemode) :!label _label
      (set `/Game/LPPGameMode_BP.CurrentTimeBetweenFalls` (`/Game/LPPGameMode_BP.TimeBetweenFasterFalls` _gamemode) _gamemode)
      (else
        (set `/Game/LPPGameMode_BP.CurrentTimeBetweenFalls` (`/Game/LPPGameMode_BP.TimeBetweenAutomaticFalls` _gamemode) _gamemode)))
    (`KismetSystemLibrary.K2_SetTimer` null "FallDownOneSpace" (`/Game/LPPGameMode_BP.CurrentTimeBetweenFalls` _gamemode))
    ;[1 1 1] decide what half to move down and move it
    (bind (_blefthalfcanmovedown _brighthalfcanmovedown) (`self.CanMoveDown`))
    (if (and _blefthalfcanmovedown _brighthalfcanmovedown)
      (`self.MoveLeftHalfDownOneSpace`)
      (`self.MoveRightHalfDownOneSpace`)
      (elif _blefthalfcanmovedown
        (`self.MoveLeftHalfDownOneSpace`)
        (elif _brighthalfcanmovedown
          (`self.MoveRightHalfDownOneSpace`)
          (else
            (`self.FinishFall`)))))))

(event `FallDownOneSpace`
  (goto _label))

(event `InputAction|Drop`
  (params (Key :type "Key Structure"))
  (:`Pressed`
    (set `/Game/LPPGameMode_BP.bIsQuadDroppingFaster` true (`self.GameMode`))
    (`self.FallDownOneSpace`)))

(fn `CanMoveDown`
  (returns (bLeftHalfCanMoveDown :type Boolean) (bRightHalfCanMoveDown :type Boolean))
  (locals (ObjectTypes :type "Array of EObjectTypeQuery Enum") (bLeftHalfCanFall :type Boolean) (bRightHalfCanFall :type Boolean))
  (bind _gamemode (`self.GameMode`))
  (bind _quad_br (`/Game/LPPGameMode_BP.Quad_BR` _gamemode))
  (bind _quad_bl (`/Game/LPPGameMode_BP.Quad_BL` _gamemode))
  (bind _returnvalue (`self.K2_GetActorLocation` _quad_bl))
  (bind _returnvalue_2 (`self.K2_GetActorLocation` _quad_br))
  (`|ExecutionSequence`
    (:`then_0`
      (bind _outhit (`KismetSystemLibrary.LineTraceSingleForObjects` _returnvalue_2 (+ _returnvalue_2 (`KismetMathLibrary.MakeVector` 0.0 0.0 (* (`/Game/LPPGameMode_BP.VerticalOffset` _gamemode) -1.0))) (`local.ObjectTypes`) false (`|MakeArray` _quad_br :!type "Actor Object Reference")))
      (`/Engine/EditorBlueprintResources/StandardMacros.IsValid` (`.HitActor` (`GameplayStatics.BreakHitResult` _outhit))
        (:`Is Valid`
          (bind _returnvalue_3 (`GameplayStatics.GetObjectClass` (`.HitActor` (`GameplayStatics.BreakHitResult` _outhit))))
          (if (or (== _returnvalue_3 "/Game/Grid_BP.Grid_BP_C") (== _returnvalue_3 "/Game/Block_BP.Block_BP_C"))
            (set `local.bRightHalfCanFall` false)
            (else
              (set `local.bRightHalfCanFall` true :!label _label))))
        (:`Is Not Valid`
          (goto _label))))
    (:`then_1`
      (bind _outhit_2 (`KismetSystemLibrary.LineTraceSingleForObjects` _returnvalue (+ _returnvalue (`KismetMathLibrary.MakeVector` 0.0 0.0 (* (`/Game/LPPGameMode_BP.VerticalOffset` _gamemode) -1.0))) (`local.ObjectTypes`) false (`|MakeArray` _quad_bl :!type "Actor Object Reference")))
      (`/Engine/EditorBlueprintResources/StandardMacros.IsValid` (`.HitActor` (`GameplayStatics.BreakHitResult` _outhit_2))
        (:`Is Valid`
          (bind _returnvalue_4 (`GameplayStatics.GetObjectClass` (`.HitActor` (`GameplayStatics.BreakHitResult` _outhit_2))))
          (if (or (== _returnvalue_4 "/Game/Grid_BP.Grid_BP_C") (== _returnvalue_4 "/Game/Block_BP.Block_BP_C"))
            (set `local.bLeftHalfCanFall` false)
            (else
              (set `local.bLeftHalfCanFall` true :!label _label_2))))
        (:`Is Not Valid`
          (goto _label_2))))
    (:`then_2`
      (return (`local.bLeftHalfCanFall`) (`local.bRightHalfCanFall`)))))

(fn `CanMoveLeft`
  (returns (bCanMove :type Boolean))
  (locals (ObjectTypes :type "Array of EObjectTypeQuery Enum"))
  (bind _gamemode (`self.GameMode`))
  (bind _quad_bl (`/Game/LPPGameMode_BP.Quad_BL` _gamemode))
  (bind _quad_tl (`/Game/LPPGameMode_BP.Quad_TL` _gamemode))
  (bind _returnvalue (`self.K2_GetActorLocation` _quad_tl))
  (bind _returnvalue_2 (`self.K2_GetActorLocation` _quad_bl))
  (`|ExecutionSequence`
    (:`then_0`
      (bind _outhit (`KismetSystemLibrary.LineTraceSingleForObjects` _returnvalue_2 (+ _returnvalue_2 (`KismetMathLibrary.MakeVector` (* -1 (`/Game/LPPGameMode_BP.HorizontalOffset` _gamemode)))) (`local.ObjectTypes`) false (`|MakeArray` _quad_bl :!type "Actor Object Reference")))
      (`/Engine/EditorBlueprintResources/StandardMacros.IsValid` (`.HitActor` (`GameplayStatics.BreakHitResult` _outhit))
        (:`Is Valid`
          (bind _returnvalue_3 (`GameplayStatics.GetObjectClass` (`.HitActor` (`GameplayStatics.BreakHitResult` _outhit))))
          (if (or (== _returnvalue_3 "/Game/Grid_BP.Grid_BP_C") (== _returnvalue_3 "/Game/Block_BP.Block_BP_C"))
            (return false)))))
    (:`then_1`
      (bind _outhit_2 (`KismetSystemLibrary.LineTraceSingleForObjects` _returnvalue (+ _returnvalue (`KismetMathLibrary.MakeVector` (* -1 (`/Game/LPPGameMode_BP.HorizontalOffset` _gamemode)))) (`local.ObjectTypes`) false (`|MakeArray` _quad_tl :!type "Actor Object Reference")))
      (`/Engine/EditorBlueprintResources/StandardMacros.IsValid` (`.HitActor` (`GameplayStatics.BreakHitResult` _outhit_2))
        (:`Is Valid`
          (bind _returnvalue_4 (`GameplayStatics.GetObjectClass` (`.HitActor` (`GameplayStatics.BreakHitResult` _outhit_2))))
          (if (or (== _returnvalue_4 "/Game/Grid_BP.Grid_BP_C") (== _returnvalue_4 "/Game/Block_BP.Block_BP_C"))
            (return false)))))
    (:`then_2`
      (return true))))

(fn `CanMoveRight`
  (returns (bCanMove :type Boolean))
  (locals (ObjectTypes :type "Array of EObjectTypeQuery Enum"))
  (bind _gamemode (`self.GameMode`))
  (bind _quad_br (`/Game/LPPGameMode_BP.Quad_BR` _gamemode))
  (bind _quad_tr (`/Game/LPPGameMode_BP.Quad_TR` _gamemode))
  (bind _returnvalue (`self.K2_GetActorLocation` _quad_tr))
  (bind _returnvalue_2 (`self.K2_GetActorLocation` _quad_br))
  (`|ExecutionSequence`
    (:`then_0`
      (bind _outhit (`KismetSystemLibrary.LineTraceSingleForObjects` _returnvalue_2 (+ _returnvalue_2 (`KismetMathLibrary.MakeVector` (`/Game/LPPGameMode_BP.HorizontalOffset` _gamemode))) (`local.ObjectTypes`) false (`|MakeArray` _quad_br :!type "Actor Object Reference")))
      (`/Engine/EditorBlueprintResources/StandardMacros.IsValid` (`.HitActor` (`GameplayStatics.BreakHitResult` _outhit))
        (:`Is Valid`
          (bind _returnvalue_3 (`GameplayStatics.GetObjectClass` (`.HitActor` (`GameplayStatics.BreakHitResult` _outhit))))
          (if (or (== _returnvalue_3 "/Game/Grid_BP.Grid_BP_C") (== _returnvalue_3 "/Game/Block_BP.Block_BP_C"))
            (return false)))))
    (:`then_1`
      (bind _outhit_2 (`KismetSystemLibrary.LineTraceSingleForObjects` _returnvalue (+ _returnvalue (`KismetMathLibrary.MakeVector` (`/Game/LPPGameMode_BP.HorizontalOffset` _gamemode))) (`local.ObjectTypes`) false (`|MakeArray` _quad_tr :!type "Actor Object Reference")))
      (`/Engine/EditorBlueprintResources/StandardMacros.IsValid` (`.HitActor` (`GameplayStatics.BreakHitResult` _outhit_2))
        (:`Is Valid`
          (bind _returnvalue_4 (`GameplayStatics.GetObjectClass` (`.HitActor` (`GameplayStatics.BreakHitResult` _outhit_2))))
          (if (or (== _returnvalue_4 "/Game/Grid_BP.Grid_BP_C") (== _returnvalue_4 "/Game/Block_BP.Block_BP_C"))
            (return false)))))
    (:`then_2`
      (return true))))

(fn `FinishFall`
  (bind _gamemode (`self.GameMode`))
  (`/Game/LPPGameMode_BP.CheckForMatchesOnAllBlocks` (`self.GameMode`))
  (set `/Game/LPPGameMode_BP.bIsQuadDroppingFaster` false _gamemode)
  (`KismetSystemLibrary.K2_SetTimer` null "FallDownOneSpace" (`/Game/LPPGameMode_BP.TimeBetweenAutomaticFalls` _gamemode))
  (`/Game/LPPGameMode_BP.SpawnNewQuad` (`self.GameMode`))
  (return))

(fn `MoveBlocksLeft`
  (bind _quadarray (`/Game/LPPGameMode_BP.GetQuadElements` (`self.GameMode`)))
  (for _array_element _quadarray
    (bind (_returnvalue_x _returnvalue_y _returnvalue_z) (`KismetMathLibrary.BreakVector` (`self.K2_GetActorLocation` _array_element)))
    (`self.K2_SetActorLocation` _array_element (`KismetMathLibrary.MakeVector` (- _returnvalue_x (`/Game/LPPGameMode_BP.HorizontalOffset` (`self.GameMode`))) _returnvalue_y _returnvalue_z) false false)))

(fn `MoveBlocksRight`
  (bind _quadarray (`/Game/LPPGameMode_BP.GetQuadElements` (`self.GameMode`)))
  (for _array_element _quadarray
    (bind (_returnvalue_x _returnvalue_y _returnvalue_z) (`KismetMathLibrary.BreakVector` (`self.K2_GetActorLocation` _array_element)))
    (`self.K2_SetActorLocation` _array_element (`KismetMathLibrary.MakeVector` (+ _returnvalue_x (`/Game/LPPGameMode_BP.HorizontalOffset` (`self.GameMode`))) _returnvalue_y _returnvalue_z) false false)))

(fn `MoveLeftHalfDownOneSpace`
  (bind _quad_bl (`/Game/LPPGameMode_BP.Quad_BL` (`self.GameMode`)))
  (bind _quad_tl (`/Game/LPPGameMode_BP.Quad_TL` (`self.GameMode`)))
  (bind (_returnvalue_x _returnvalue_y _returnvalue_z) (`KismetMathLibrary.BreakVector` (`self.K2_GetActorLocation` _quad_tl)))
  (bind (_returnvalue_x_2 _returnvalue_y_2 _returnvalue_z_2) (`KismetMathLibrary.BreakVector` (`self.K2_GetActorLocation` _quad_bl)))
  (`|ExecutionSequence`
    (:`then_0`
      (`self.K2_SetActorLocation` _quad_bl (`KismetMathLibrary.MakeVector` _returnvalue_x_2 _returnvalue_y_2 (- _returnvalue_z_2 (`/Game/LPPGameMode_BP.HorizontalOffset` (`self.GameMode`)))) false false))
    (:`then_1`
      (`self.K2_SetActorLocation` _quad_tl (`KismetMathLibrary.MakeVector` _returnvalue_x _returnvalue_y (- _returnvalue_z (`/Game/LPPGameMode_BP.HorizontalOffset` (`self.GameMode`)))) false false))
    (:`then_2`
      (return))))

(fn `MoveRightHalfDownOneSpace`
  (bind _quad_br (`/Game/LPPGameMode_BP.Quad_BR` (`self.GameMode`)))
  (bind _quad_tr (`/Game/LPPGameMode_BP.Quad_TR` (`self.GameMode`)))
  (bind (_returnvalue_x _returnvalue_y _returnvalue_z) (`KismetMathLibrary.BreakVector` (`self.K2_GetActorLocation` _quad_tr)))
  (bind (_returnvalue_x_2 _returnvalue_y_2 _returnvalue_z_2) (`KismetMathLibrary.BreakVector` (`self.K2_GetActorLocation` _quad_br)))
  (`|ExecutionSequence`
    (:`then_0`
      (`self.K2_SetActorLocation` _quad_br (`KismetMathLibrary.MakeVector` _returnvalue_x_2 _returnvalue_y_2 (- _returnvalue_z_2 (`/Game/LPPGameMode_BP.HorizontalOffset` (`self.GameMode`)))) false false))
    (:`then_1`
      (`self.K2_SetActorLocation` _quad_tr (`KismetMathLibrary.MakeVector` _returnvalue_x _returnvalue_y (- _returnvalue_z (`/Game/LPPGameMode_BP.HorizontalOffset` (`self.GameMode`)))) false false))
    (:`then_2`
      (return))))

(fn `RotateBlocksCCW`
  (locals (OldColorBL :type Boolean) (OldColorBR :type Boolean))
  (bind _gamemode (`self.GameMode`))
  (set `local.OldColorBR` (`/Game/Block_BP.bIsColor1` (`/Game/LPPGameMode_BP.Quad_BR` (`self.GameMode`))))
  (`|ExecutionSequence`
    (:`then_0`
      (set `/Game/Block_BP.bIsColor1` (`/Game/Block_BP.bIsColor1` (`/Game/LPPGameMode_BP.Quad_BL` _gamemode)) (`/Game/LPPGameMode_BP.Quad_BR` _gamemode)))
    (:`then_1`
      (set `/Game/Block_BP.bIsColor1` (`/Game/Block_BP.bIsColor1` (`/Game/LPPGameMode_BP.Quad_TL` _gamemode)) (`/Game/LPPGameMode_BP.Quad_BL` _gamemode)))
    (:`then_2`
      (set `/Game/Block_BP.bIsColor1` (`/Game/Block_BP.bIsColor1` (`/Game/LPPGameMode_BP.Quad_TR` _gamemode)) (`/Game/LPPGameMode_BP.Quad_TL` _gamemode)))
    (:`then_3`
      (set `/Game/Block_BP.bIsColor1` (`local.OldColorBR`) (`/Game/LPPGameMode_BP.Quad_TR` _gamemode)))
    (:`then_4`
      (bind _quadarray (`/Game/LPPGameMode_BP.GetQuadElements` _gamemode))
      (for _array_element _quadarray
        (`/Game/Block_BP.SetColorByBoolean` _array_element))
      (return))))

(fn `RotateBlocksCW`
  (locals (OldColorBL :type Boolean))
  (bind _gamemode (`self.GameMode`))
  (set `local.OldColorBL` (`/Game/Block_BP.bIsColor1` (`/Game/LPPGameMode_BP.Quad_BL` (`self.GameMode`))))
  (`|ExecutionSequence`
    (:`then_0`
      (set `/Game/Block_BP.bIsColor1` (`/Game/Block_BP.bIsColor1` (`/Game/LPPGameMode_BP.Quad_BR` _gamemode)) (`/Game/LPPGameMode_BP.Quad_BL` _gamemode)))
    (:`then_1`
      (set `/Game/Block_BP.bIsColor1` (`/Game/Block_BP.bIsColor1` (`/Game/LPPGameMode_BP.Quad_TR` _gamemode)) (`/Game/LPPGameMode_BP.Quad_BR` _gamemode)))
    (:`then_2`
      (set `/Game/Block_BP.bIsColor1` (`/Game/Block_BP.bIsColor1` (`/Game/LPPGameMode_BP.Quad_TL` _gamemode)) (`/Game/LPPGameMode_BP.Quad_TR` _gamemode)))
    (:`then_3`
      (set `/Game/Block_BP.bIsColor1` (`local.OldColorBL`) (`/Game/LPPGameMode_BP.Quad_TL` _gamemode)))
    (:`then_4`
      (bind _quadarray (`/Game/LPPGameMode_BP.GetQuadElements` _gamemode))
      (for _array_element _quadarray
        (`/Game/Block_BP.SetColorByBoolean` _array_element))
      (return))))

(fn `UserConstructionScript`
  (bind _aslppgame_mode_bp (cast `/Game/LPPGameMode_BP` (`GameplayStatics.GetGameMode`)))
  (set `self.GameMode` _aslppgame_mode_bp))