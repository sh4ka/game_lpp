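; TimerBar_BP is the timer bar that sweeps horizontally across the block grid, highlighting blocks it passes.
; Tick moves it by HorizontalVelocity scaled by delta time.
; Mesh overlaps highlight blocks in a specific state, while hitting the grid's right collision box teleports the bar back to the game mode's starting location.
; Column checker overlaps are ignored, and ScanColumnForBlocks is an empty stub.
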(event `self.ReceiveBeginPlay`
  (bind _aslppgame_mode_bp (cast `/Game/LPPGameMode_BP` (`GameplayStatics.GetGameMode`)))
  (set `self.game mode` _aslppgame_mode_bp))

(event `self.ReceiveTick`
  (params (DeltaSeconds :type "Float (single-precision)"))
  (`self.K2_SetActorLocation` (+ (`self.K2_GetActorLocation`) (* (`self.HorizontalVelocity`) DeltaSeconds))))

(event `self.TimerBarMesh.OnComponentBeginOverlap`
  (params (OverlappedComponent :type "PrimitiveComponent Object Reference") (OtherActor :type "Actor Object Reference") (OtherComp :type "PrimitiveComponent Object Reference") (OtherBodyIndex :type Integer) (bFromSweep :type Boolean) (SweepResult :type "HitResult Structure (by ref)"))
  (bind _returnvalue (`KismetSystemLibrary.IsValid` OtherActor))
  (if (and _returnvalue (== (`GameplayStatics.GetObjectClass` OtherActor) "/Game/Block_BP.Block_BP_C"))
    (bind _asblock_bp (cast `/Game/Block_BP` OtherActor))
    (if (`|EnumEquality` (`/Game/Block_BP.MyState` _asblock_bp) "NewEnumerator1")
      (`/Game/Block_BP.BecomeHighlighted` _asblock_bp))
    (elif (and _returnvalue (== (`GameplayStatics.GetObjectClass` OtherActor) "/Game/Column_Checker_BP.Column_Checker_BP_C"))
      _
      (elif (== OtherComp (`/Game/Grid_BP.RightCollisionBox` (`self.Grid`)))
        (`self.K2_SetActorLocation` (`/Game/LPPGameMode_BP.TimerBarStartingLocation` (`self.game mode`)))))))

(fn `ScanColumnForBlocks`)

(fn `UserConstructionScript`)