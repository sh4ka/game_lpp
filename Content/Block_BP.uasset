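; Two-color puzzle board block that detects same-colored 2x2 squares and changes look as it becomes matched, then highlighted.
; DetermineMatches line-traces eight neighbors at game-mode offsets, counts matching corner squares and triggers BecomeMatched.
; Timelines interpolate a dynamic material between state looks and drive a SphereKey morph, with highlighting swapping in a cubesphere skeletal mesh.
; Clearing destroys the actor, while unmatching and dropping are empty stubs.
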(event `Color1Transition_UnmatchedToMatched`
  (set `self.StartingMattInst` (`self.MyMattInst_Dyn`))
  (if (`self.bIsColor1`)
    (set `self.TargetMattInst` "/Game/StaticMeshes/Materials/BlockColor1_Matched_Inst.BlockColor1_Matched_Inst")
    (bind (_direction _interpolationpercent) (`Timeline|ColorTransition` :!via `PlayFromStart` :!label _label)
      (:`Update`
        (`MaterialInstanceDynamic.K2_InterpolateMaterialInstanceParams` (`self.MyMattInst_Dyn`) (`self.StartingMattInst`) (`self.TargetMattInst`) _interpolationpercent)
        (`SkeletalMeshComponent.SetMorphTarget` (`self.SkeletalMesh`) "SphereKey" _interpolationpercent true)))
    (else
      (set `self.TargetMattInst` "/Game/StaticMeshes/Materials/BlockColor0_Matched_Inst.BlockColor0_Matched_Inst")
      (goto _label :!via `PlayFromStart`))))

(event `ColorTransition_MatchedToHighlighted`
  (set `self.StartingMattInst` (`self.MyMattInst_Dyn`))
  (if (`self.bIsColor1`)
    (set `self.TargetMattInst` "/Game/StaticMeshes/Materials/BlockColor1_Highlighted_Inst.BlockColor1_Highlighted_Inst")
    (bind (_direction _interpolationpercent) (`Timeline|Timeline_0` :!via `PlayFromStart` :!label _label_2)
      (:`Update`
        (`MaterialInstanceDynamic.K2_InterpolateMaterialInstanceParams` (`self.MyMattInst_Dyn`) (`self.StartingMattInst`) (`self.TargetMattInst`) _interpolationpercent)
        (`SkeletalMeshComponent.SetMorphTarget` (`self.SkeletalMesh`) "SphereKey" _interpolationpercent true)))
    (else
      (set `self.TargetMattInst` "/Game/StaticMeshes/Materials/BlockColor0_Highlighted_Inst.BlockColor0_Highlighted_Inst")
      (goto _label_2 :!via `PlayFromStart`))))

(fn `BecomeHighlighted`
  (bind _skeletalmesh (`self.SkeletalMesh`))
  (set `self.MyState` "NewEnumerator2")
  (`SkinnedMeshComponent.SetSkinnedAssetAndUpdate` _skeletalmesh "/Game/StaticMeshes/cubesphere.cubesphere" true)
  (`PrimitiveComponent.SetMaterial` _skeletalmesh 0 (`self.MyMattInst_Dyn`))
  (`SceneComponent.SetVisibility` (`self.BlockMesh`) false false)
  (`self.ColorTransition_MatchedToHighlighted`))

(fn `BecomeMatched`
  (set `self.MyState` "NewEnumerator1")
  (`self.Color1Transition_UnmatchedToMatched`))

(fn `BecomeUnmatched`)

(fn `ClearSelfFromTheBoard`
  (`self.K2_DestroyActor`)
  (return))

(fn `DetermineMatches`
  (returns (NumberOfMatches :type Integer))
  (locals (ObjectTypes :type "Array of EObjectTypeQuery Enum") (ArrayOfComparisonResults :type "Array of Boolean") (OffsetsArray :type "Array of Vector Structure") (NumMatches :type Integer))
  (bind _returnvalue (`self.K2_GetActorLocation`))
  (bind _gamemode (`self.GameMode`))
  (bind _arrayofcomparisonresults (`local.ArrayOfComparisonResults`))
  (bind _arrayofcomparisonresults_2 (`local.ArrayOfComparisonResults`))
  (bind _arrayofcomparisonresults_3 (`local.ArrayOfComparisonResults`))
  (bind _arrayofcomparisonresults_4 (`local.ArrayOfComparisonResults`))
  (bind _verticaloffset (`/Game/LPPGameMode_BP.VerticalOffset` _gamemode))
  (bind _horizontaloffset (`/Game/LPPGameMode_BP.HorizontalOffset` _gamemode))
  (bind _returnvalue_2 (* -1 _horizontaloffset))
  (bind _returnvalue_3 (* -1 _verticaloffset))
  (`|ExecutionSequence`
    (:`then_0`
      (set `local.OffsetsArray` (`|MakeArray` (`KismetMathLibrary.MakeVector` 0.0 0.0 _horizontaloffset) (`KismetMathLibrary.MakeVector` _horizontaloffset 0.0 _verticaloffset) (`KismetMathLibrary.MakeVector` _horizontaloffset) (`KismetMathLibrary.MakeVector` _horizontaloffset 0.0 _returnvalue_3) (`KismetMathLibrary.MakeVector` 0.0 0.0 _returnvalue_3) (`KismetMathLibrary.MakeVector` _returnvalue_2 0.0 _returnvalue_3) (`KismetMathLibrary.MakeVector` _returnvalue_2) (`KismetMathLibrary.MakeVector` _returnvalue_2 0.0 _verticaloffset)))
      (for (_array_element _array_index) (`local.OffsetsArray`)
        (bind _outhit (`KismetSystemLibrary.LineTraceSingleForObjects` _returnvalue (+ _returnvalue _array_element) (`local.ObjectTypes`)))
        (`/Engine/EditorBlueprintResources/StandardMacros.IsValid` (`.HitActor` (`GameplayStatics.BreakHitResult` _outhit))
          (:`Is Valid`
            (bind _asblock_bp (cast `/Game/Block_BP` (`.HitActor` (`GameplayStatics.BreakHitResult` _outhit))))
            (`KismetArrayLibrary.Array_Set` (`local.ArrayOfComparisonResults`) _array_index (== (`/Game/Block_BP.bIsColor1` _asblock_bp) (`self.bIsColor1`)))))))
    (:`then_1`
      (if (and (`|GetArrayItem` _arrayofcomparisonresults_2) (`|GetArrayItem` _arrayofcomparisonresults_2 1) (`|GetArrayItem` _arrayofcomparisonresults_2 2))
        (`/Engine/EditorBlueprintResources/StandardMacros.IncrementInt` (`local.NumMatches`))))
    (:`then_2`
      (if (and (`|GetArrayItem` _arrayofcomparisonresults_3 2) (`|GetArrayItem` _arrayofcomparisonresults_3 3) (`|GetArrayItem` _arrayofcomparisonresults_3 4))
        (`/Engine/EditorBlueprintResources/StandardMacros.IncrementInt` (`local.NumMatches`))))
    (:`then_3`
      (if (and (`|GetArrayItem` _arrayofcomparisonresults_4 4) (`|GetArrayItem` _arrayofcomparisonresults_4 5) (`|GetArrayItem` _arrayofcomparisonresults_4 6))
        (`/Engine/EditorBlueprintResources/StandardMacros.IncrementInt` (`local.NumMatches`))))
    (:`then_4`
      (if (and (`|GetArrayItem` _arrayofcomparisonresults 6) (`|GetArrayItem` _arrayofcomparisonresults 7) (`|GetArrayItem` _arrayofcomparisonresults))
        (`/Engine/EditorBlueprintResources/StandardMacros.IncrementInt` (`local.NumMatches`))))
    (:`then_5`
      (if (> (`local.NumMatches`) 0)
        (if (`|EnumEquality` (`self.MyState`) "NewEnumerator0")
          (`self.BecomeMatched`)))
      (return (`local.NumMatches`)))))

(fn `DropAsFarAsPossible`)

(fn `SetColorByBoolean`
  (bind _blockmesh (`self.BlockMesh`))
  (if (`self.bIsColor1`)
    (bind _returnvalue (`KismetMaterialLibrary.CreateDynamicMaterialInstance` "/Game/StaticMeshes/Materials/BlockColor1_Unmatched_Inst.BlockColor1_Unmatched_Inst"))
    (bind _output_get (set `self.MyMattInst_Dyn` _returnvalue))
    (`PrimitiveComponent.SetMaterial` _blockmesh 0 _output_get)
    (else
      (bind _returnvalue_2 (`KismetMaterialLibrary.CreateDynamicMaterialInstance` "/Game/StaticMeshes/Materials/BlockColor0_Unmatched_Inst.BlockColor0_Unmatched_Inst"))
      (bind _output_get_2 (set `self.MyMattInst_Dyn` _returnvalue_2))
      (`PrimitiveComponent.SetMaterial` _blockmesh 0 _output_get_2)))
  (return))

(fn `UserConstructionScript`
  (`self.SetColorByBoolean`)
  (bind _aslppgame_mode_bp (cast `/Game/LPPGameMode_BP` (`GameplayStatics.GetGameMode`)))
  (set `self.GameMode` _aslppgame_mode_bp))